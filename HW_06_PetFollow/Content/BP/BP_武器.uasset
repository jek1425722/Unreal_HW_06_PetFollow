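; Weapon Blueprint that fires automatically while the fire input is held and tracks magazine and reserve ammo.
; Firing loops on a Delay while ammo remains, spawning BP_子彈 at the muzzle socket, passing it weapon damage, emitting a muzzle flash and decrementing the magazine.
; Custom event 換彈匣 refills the magazine from reserve, limited to what remains.
; Custom event 補充子彈 adds one magazine's worth to reserve, clamped to its maximum.
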(event Custom|換彈匣
  ;[0.3278 0.4852 1] 計算要補充幾顆子彈
  (Variables|Default|Set要補充的子彈數量 (- (Variables|Default|Get彈匣尺寸) (Variables|Default|Get目前子彈數量))) ; 計算要補充的彈匣數量\n例：目前10 彈匣30 所以要補充20
  ;[0.3278 0.4852 1] 判斷總數是否>=要補充的數量
  (if (>= (Variables|Default|Get子彈總數) (Variables|Default|Get要補充的子彈數量))
    _
    (else
      ;[0.3278 0.4852 1] 總數<要補充的數量：把剩餘總數補充
      (Variables|Default|Set要補充的子彈數量 (Variables|Default|Get子彈總數))))
  ;[0.3278 0.4852 1] 目前子彈以及總數更新
  (Variables|Default|Set目前子彈數量 (+ (Variables|Default|Get目前子彈數量) (Variables|Default|Get要補充的子彈數量))) ; 補充子彈數量\n例：目前10 要補充為20 補充後 目前為30
  (Variables|Default|Set子彈總數 (- (Variables|Default|Get子彈總數) (Variables|Default|Get要補充的子彈數量))) ; 扣除子彈總數\n例：總數20 要補充為20 補充後 總數為0
)

(event Custom|補充子彈
  ;[1 1 1] 補充子彈
  (bind _output_get (Variables|Default|Set子彈總數 (+ (Variables|Default|Get子彈總數) (Variables|Default|Get彈匣尺寸)))) ; 子彈總數 + 彈匣尺寸
  (Variables|Default|Set子彈總數 (Math|Integer|Clamp(Integer) _output_get 0 (Variables|Default|Get子彈上限))))

(event Input|ActionEvents|InputAction開槍
  (params (Key :type Key%20Structure :default "None"))
  (bind _武器模型 (Variables|Default|Get武器模型))
  (bind _returnvalue (Transformation|GetSocketRotation _武器模型 "None"))
  ;[1 1 1] 開槍
  (:Pressed
    (Variables|Default|Set開槍中 true)
    (if (and (> (Variables|Default|Get目前子彈數量) 0) (Variables|Default|Get開槍中)) :!label _label ; 當目前子彈>0才可以開槍
      (bind _returnvalue_2 (Game|SpawnActorfromClass "/Game/BP/BP_子彈.BP_子彈_C" (Transformation|GetSocketTransform (Variables|Default|Get武器模型) "子彈插槽" "RTS_World") "Undefined" 0 0)) ; 生成子彈藍圖
      (Variables|/Game/BP/BP_子彈.BP_子彈_C|Set目前武器傷害 _returnvalue_2 (Variables|Default|Get武器傷害)) ; 將武器傷害傳給子彈
      (Effects|SpawnEmitteratLocation "/Game/InfinityBladeEffects/Effects/FX_Monsters/FX_Monster_Gruntling/Master/P_BackPack_MuzzleFlash.P_BackPack_MuzzleFlash" (Transformation|GetSocketLocation _武器模型 "子彈插槽") (Math|Rotator|MakeRotator (+ (.roll _returnvalue) 9e+01) (.pitch _returnvalue) (+ (.yaw _returnvalue) 9e+01)) "0.080000,0.080000,0.080000") ; 生成粒子在指定座標上
      (Variables|Default|Set目前子彈數量 (- (Variables|Default|Get目前子彈數量) 1)) ; 開槍後子彈減一
      (Utilities|FlowControl|Delay (Variables|Default|Get開槍間隔))
      (goto _label)))
  (:Released
    (Variables|Default|Set開槍中 false)))

(fn ConstructionScript)