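; BP_遊戲模式 (game mode, by its name) runs a minute-and-second countdown meant to pause the game when time runs out.
; Tick feeds a one-second Delay, which throttles the decrement of 秒 (seconds) to roughly once per second.
; When seconds drop below zero, they reset to 60 and 分 (minutes) decrements if positive.
; At zero minutes, the pause requires seconds to equal 59, which that reset prevents.
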(event EventTick
  (params (DeltaSeconds :type Float%20%28single-precision%29))
  ;[0.6897 0.3958 1] 倒數系統
  ;;[1 1 1] 每秒秒數減一
  (Utilities|FlowControl|Delay 1.0) ; 延遲：等待所設定的時間執行後面的節點
  (bind _output_get (Variables|Default|Set秒 (- (Variables|Default|Get秒) 1)))
  ;;[1 1 1] 當秒數低於0就把秒數設定為59秒
  (if (< _output_get 0) ; 判斷：\n當布林值為正確\n從true出去\n為錯誤\n從false出去
    (Variables|Default|Set秒 60)
    ;;[1 1 1] 分大於0時分減1
    (if (> (Variables|Default|Get分) 0)
      (Variables|Default|Set分 (- (Variables|Default|Get分) 1))
      (else
        ;;[1 1 1] 分為0時秒等於59 就代表已經沒有時間 將秒設為0並暫停遊戲
        (if (== (Variables|Default|Get秒) 59)
          (Variables|Default|Set秒 0)
          (Game|SetGamePaused true))))))

(fn ConstructionScript)